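; BP_Key is a key pickup actor that records the acquired key in the game mode when interacted with.
; On BeginPlay it caches BP_GameMode, then Interact overwrites that game mode's Keys value with its own KeyNumber.
; It prints an acquisition message using the matching entry in Names, then destroys itself.
; The construction script applies the Material variable to the Key component, allowing a different look per key.
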(event `self.ReceiveBeginPlay`
  (bind _asbp_game_mode (cast `/Game/LabWork1/BP_GameMode` (`GameplayStatics.GetGameMode`)))
  (set `self.As BP Game Mode` _asbp_game_mode))

(event `/Game/LabWork1/BPI_Interactable.Interact`
  (bind _output_get (set `/Game/LabWork1/BP_GameMode.Keys` (`self.Key Number`) (`self.As BP Game Mode`)))
  (`KismetSystemLibrary.PrintString` (`KismetStringLibrary.Concat_StrStr` "Key" (`|GetArrayItem` (`self.Names`) _output_get) "Acquired"))
  (`self.K2_DestroyActor`))

(fn `UserConstructionScript`
  (`PrimitiveComponent.SetMaterial` (`self.Key`) 0 (`self.Material`)))