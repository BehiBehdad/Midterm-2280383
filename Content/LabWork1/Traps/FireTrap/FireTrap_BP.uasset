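; Fire trap actor that burns the third-person player character while it stands inside the fire area.
; Overlapping FireArea sets an in-radius flag and subtracts a fixed chunk of Health, repeating through a Delay loop until the character leaves.
; When Health drops to zero or below, the loop stops and calls Ragdoll on player 0's character.
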(event `self.Fire Area.OnComponentBeginOverlap`
  (params (OverlappedComponent :type "PrimitiveComponent Object Reference") (OtherActor :type "Actor Object Reference") (OtherComp :type "PrimitiveComponent Object Reference") (OtherBodyIndex :type Integer) (bFromSweep :type Boolean) (SweepResult :type "HitResult Structure (by ref)"))
  (bind _asbp_third_person_character (cast `/Game/LabWork1/Swat/BP_ThirdPersonCharacter` OtherActor))
  (set `self.PlayerInRadius` true)
  (bind _output_get (set `/Game/LabWork1/Swat/BP_ThirdPersonCharacter.Health` (- (`/Game/LabWork1/Swat/BP_ThirdPersonCharacter.Health` _asbp_third_person_character) 5.0) _asbp_third_person_character :!label _label))
  (if (<= _output_get 0.0)
    (bind _asbp_third_person_character_2 (cast `/Game/LabWork1/Swat/BP_ThirdPersonCharacter` (`GameplayStatics.GetPlayerCharacter` 0)))
    (`/Game/LabWork1/Swat/BP_ThirdPersonCharacter.Ragdoll` _asbp_third_person_character_2)
    (else
      (`KismetSystemLibrary.Delay` 0.5)
      (if (`self.PlayerInRadius`)
        (goto _label)))))

(event `self.Fire Area.OnComponentEndOverlap`
  (params (OverlappedComponent :type "PrimitiveComponent Object Reference") (OtherActor :type "Actor Object Reference") (OtherComp :type "PrimitiveComponent Object Reference") (OtherBodyIndex :type Integer))
  (cast `/Game/LabWork1/Swat/BP_ThirdPersonCharacter` OtherActor)
  (set `self.PlayerInRadius` false))

(fn `UserConstructionScript`)