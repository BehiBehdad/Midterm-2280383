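; Pendulum trap actor that swings its mesh back and forth and damages the third-person character on contact.
; A timeline lerps mesh pitch between two extremes, alternating forward and reverse endlessly from BeginPlay.
; Collision overlap launches the character toward the trap's origin with an upward boost and subtracts a fixed amount of Health.
; At zero or below, player 0's character ragdolls and the trap destroys itself.
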(event `self.ReceiveBeginPlay`
  (bind (_direction _movement) (`Timeline|Movement Time` :!label _label)
    (:`Update`
      (`SceneComponent.K2_SetRelativeRotation` (`self.Mesh`) (`KismetMathLibrary.RLerp` (struct :`Roll` -60.0) (struct :`Roll` 60.0) _movement) false false))
    (:`Finished`
      (if (`|EnumEquality` _direction "Forward")
        (goto _label :!via `Reverse`)
        (else
          (goto _label :!via `PlayFromStart`))))))

(event `self.Collision.OnComponentBeginOverlap`
  (params (OverlappedComponent :type "PrimitiveComponent Object Reference") (OtherActor :type "Actor Object Reference") (OtherComp :type "PrimitiveComponent Object Reference") (OtherBodyIndex :type Integer) (bFromSweep :type Boolean) (SweepResult :type "HitResult Structure (by ref)"))
  (bind _asbp_third_person_character (cast `/Game/LabWork1/Swat/BP_ThirdPersonCharacter` OtherActor))
  (`Character.LaunchCharacter` _asbp_third_person_character (+ (* (`KismetMathLibrary.Normal` (- (`self.K2_GetActorLocation`) (`self.K2_GetActorLocation` _asbp_third_person_character))) 1500.0) (* (`self.GetActorUpVector`) 150.0)) false false)
  (bind _output_get (set `/Game/LabWork1/Swat/BP_ThirdPersonCharacter.Health` (- (`/Game/LabWork1/Swat/BP_ThirdPersonCharacter.Health` _asbp_third_person_character) 70.0) _asbp_third_person_character))
  (if (<= _output_get 0.0)
    (bind _asbp_third_person_character_2 (cast `/Game/LabWork1/Swat/BP_ThirdPersonCharacter` (`GameplayStatics.GetPlayerCharacter` 0)))
    (`/Game/LabWork1/Swat/BP_ThirdPersonCharacter.Ragdoll` _asbp_third_person_character_2)
    (`self.K2_DestroyActor`)))

(fn `UserConstructionScript`)